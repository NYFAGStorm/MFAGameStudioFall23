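; Prototype player-flown dragon pawn with physics-based flight, keyboard throttle, pitch, yaw and roll, and a looping placeholder animation.
; Key flags feed fixed-interval timer functions that ramp throttle and self-centering axis amounts, applying axis torques to PhysicsRoot.
; Tick damps spin, adds gravity and throttle-based lift, eases velocity toward forward thrust, then blends momentum toward the nose via ForwardCheat.
; Orientation settling is unfinished and applies zero torque.
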(event EventTick
  (params (DeltaSeconds :type Float%20%28single-precision%29))
  ;[0.3804 0.3294 0.2353] Settle Torque
  (CallFunction|SettleTorque)
  ;[0.3804 0.3294 0.2353] Settle Orientation (wip)
  (CallFunction|SettleOrientation)
  ;[0.381 0.3278 0.2358] Gravity Simulated
  (Physics|AddForce (Variables|Default|GetPhysics%20Root) "0.000000,0.000000,-900.000000" "None" true)
  ;[0.3804 0.3294 0.2353] Thrust Forward
  (CallFunction|CalculateSpeed)
  ;[0.3804 0.3294 0.2353] Simulated Lift
  (CallFunction|CalculateLift)
  ;[0.3804 0.3294 0.2353] Cheat Velocity Forward
  (CallFunction|CheatForwardVelocity))

(event EventBeginPlay
  (bind _dragonmesh (Variables|Default|GetDragonMesh))
  ;[0.381 0.3278 0.2358] Flight Control Config
  (Utilities|Time|SetTimerbyFunctionName 0 "ThrottleControl" 0.02 true)
  (Utilities|Time|SetTimerbyFunctionName 0 "PitchControl" 0.02 true)
  (Utilities|Time|SetTimerbyFunctionName 0 "YawControl" 0.02 true)
  (Utilities|Time|SetTimerbyFunctionName 0 "RollControl" 0.02 true)
  ;[0.3804 0.3294 0.2353] TEMP Dragon Config
  (Transformation|SetRelativeLocation _dragonmesh "-40.000000,0.000000,-618.000000" false false)
  (Components|Animation|PlayAnimation _dragonmesh "/Game/Dragon12/Animations/Dragon/Anim_Dragon12_Attack_Base3b.Anim_Dragon12_Attack_Base3b" true))

(event Input|KeyboardEvents|LeftShift
  (params (Key :type Key%20Structure :default "None"))
  ;[0.381 0.3278 0.2358] Throttle Input
  (:Pressed
    (Variables|Default|SetThrottleUp true))
  (:Released
    (Variables|Default|SetThrottleUp false)))

(event Input|KeyboardEvents|LeftCtrl
  (params (Key :type Key%20Structure :default "None"))
  ;[0.381 0.3278 0.2358] Throttle Input
  (:Pressed
    (Variables|Default|SetThrottleDown true))
  (:Released
    (Variables|Default|SetThrottleDown false)))

(event Input|KeyboardEvents|W
  (params (Key :type Key%20Structure :default "None"))
  ;[0.3804 0.3294 0.2353] Pitch Input
  (:Pressed
    (Variables|Default|SetPitchDown true))
  (:Released
    (Variables|Default|SetPitchDown false)))

(event Input|KeyboardEvents|S
  (params (Key :type Key%20Structure :default "None"))
  ;[0.3804 0.3294 0.2353] Pitch Input
  (:Pressed
    (Variables|Default|SetPitchUp true))
  (:Released
    (Variables|Default|SetPitchUp false)))

(event Input|KeyboardEvents|A
  (params (Key :type Key%20Structure :default "None"))
  ;[0.381 0.3278 0.2358] Yaw Input
  (:Pressed
    (Variables|Default|SetYawLeft true))
  (:Released
    (Variables|Default|SetYawLeft false)))

(event Input|KeyboardEvents|D
  (params (Key :type Key%20Structure :default "None"))
  ;[0.381 0.3278 0.2358] Yaw Input
  (:Pressed
    (Variables|Default|SetYawRight true))
  (:Released
    (Variables|Default|SetYawRight false)))

(event Input|KeyboardEvents|Q
  (params (Key :type Key%20Structure :default "None"))
  ;[0.3804 0.3294 0.2353] Roll Input
  (:Pressed
    (Variables|Default|SetRollCounterClock true))
  (:Released
    (Variables|Default|SetRollCounterClock false)))

(event Input|KeyboardEvents|E
  (params (Key :type Key%20Structure :default "None"))
  ;[0.3804 0.3294 0.2353] Roll Input
  (:Pressed
    (Variables|Default|SetRollClockwise true))
  (:Released
    (Variables|Default|SetRollClockwise false)))

(fn ConstructionScript)

(fn ThrottleControl
  (if (Variables|Default|GetThrottleUp)
    (bind _result (Math|Integer|IncrementInt (Variables|Default|GetThrottleAmount))
      (:%20%20
        (bind _output_get (Variables|Default|SetThrottleAmount (Math|Integer|Clamp(Integer) _result 0 100)))
        (Development|PrintText (Utilities|Text|FormatText "Speed {0}" (Utilities|Text|ToText(Integer) _output_get)))))
    (elif (Variables|Default|GetThrottleDown)
      (bind _result_2 (Math|Integer|DecrementInt (Variables|Default|GetThrottleAmount))
        (:%20%20
          (bind _output_get_2 (Variables|Default|SetThrottleAmount (Math|Integer|Clamp(Integer) _result_2 0 100)))
          (Development|PrintText (Utilities|Text|FormatText "Speed {0}" (Utilities|Text|ToText(Integer) _output_get_2))))))))

(fn PitchControl
  (bind _control_attack (Variables|Default|GetControl%20Attack))
  (if (Variables|Default|GetPitchDown)
    (bind _output_get (Variables|Default|SetPitchAmount (Math|Float|Clamp(Float) (+ (Variables|Default|GetPitchAmount) _control_attack) -1.0) :!label _label))
    (Development|PrintText (Utilities|Text|FormatText "Pitch {0}" _output_get) true true "(R=0.166667,G=0.000000,B=1.000000,A=1.000000)")
    (Class|PrimitiveComponent|AddTorqueinDegrees (Variables|Default|GetPhysics%20Root) (Math|Vector|Lerp(Vector) "0, 0, 0" (* (Math|Vector|GetRightVector (Variables|Default|GetPhysics%20Root)) (* (Variables|Default|GetPitchAmount) (Variables|Default|GetAirControl))) 0.1) "None" true :!label _label_2)
    (elif (Variables|Default|GetPitchUp)
      (bind _output_get_2 (Variables|Default|SetPitchAmount (Math|Float|Clamp(Float) (+ (Variables|Default|GetPitchAmount) (Utilities|Invert _control_attack)) -1.0) :!label _label_3))
      (Development|PrintText (Utilities|Text|FormatText "Pitch {0}" _output_get_2) true true "(R=0.166667,G=0.000000,B=1.000000,A=1.000000)")
      (goto _label_2)
      (elif (< (Variables|Default|GetPitchAmount) -0.01)
        (goto _label)
        (elif (> (Variables|Default|GetPitchAmount) 0.01)
          (goto _label_3))))))

(fn YawControl
  (bind _control_attack (Variables|Default|GetControl%20Attack))
  (if (Variables|Default|GetYawRight)
    (bind _output_get (Variables|Default|SetYawAmount (Math|Float|Clamp(Float) (+ (Variables|Default|GetYawAmount) _control_attack) -1.0) :!label _label))
    (Development|PrintText (Utilities|Text|FormatText "Yaw {0}" _output_get) true true "(R=1.000000,G=0.000380,B=1.000000,A=1.000000)")
    (Class|PrimitiveComponent|AddTorqueinDegrees (Variables|Default|GetPhysics%20Root) (Math|Vector|Lerp(Vector) "0, 0, 0" (* (Math|Vector|GetUpVector (Variables|Default|GetPhysics%20Root)) (* (Variables|Default|GetYawAmount) (Variables|Default|GetAirControl))) 0.1) "None" true :!label _label_2)
    (elif (Variables|Default|GetYawLeft)
      (bind _output_get_2 (Variables|Default|SetYawAmount (Math|Float|Clamp(Float) (+ (Variables|Default|GetYawAmount) (Utilities|Invert _control_attack)) -1.0) :!label _label_3))
      (Development|PrintText (Utilities|Text|FormatText "Yaw {0}" _output_get_2) true true "(R=1.000000,G=0.000000,B=1.000000,A=1.000000)")
      (goto _label_2)
      (elif (< (Variables|Default|GetYawAmount) -0.01)
        (goto _label)
        (elif (> (Variables|Default|GetYawAmount) 0.01)
          (goto _label_3))))))

(fn RollControl
  (bind _control_attack (Variables|Default|GetControl%20Attack))
  (if (Variables|Default|GetRollCounterClock)
    (bind _output_get (Variables|Default|SetRollAmount (Math|Float|Clamp(Float) (+ (Variables|Default|GetRollAmount) _control_attack) -1.0) :!label _label))
    (Development|PrintText (Utilities|Text|FormatText "Roll {0}" _output_get) true true "(R=1.000000,G=0.000380,B=0.166983,A=1.000000)")
    (Class|PrimitiveComponent|AddTorqueinDegrees (Variables|Default|GetPhysics%20Root) (Math|Vector|Lerp(Vector) "0, 0, 0" (* (Math|Vector|GetForwardVector (Variables|Default|GetPhysics%20Root)) (* (Variables|Default|GetRollAmount) (Variables|Default|GetAirControl))) 0.1) "None" true :!label _label_2)
    (elif (Variables|Default|GetRollClockwise)
      (bind _output_get_2 (Variables|Default|SetRollAmount (Math|Float|Clamp(Float) (+ (Variables|Default|GetRollAmount) (Utilities|Invert _control_attack)) -1.0) :!label _label_3))
      (Development|PrintText (Utilities|Text|FormatText "Roill {0}" _output_get_2) true true "(R=1.000000,G=0.000000,B=0.166667,A=1.000000)")
      (goto _label_2)
      (elif (< (Variables|Default|GetRollAmount) -0.01)
        (goto _label)
        (elif (> (Variables|Default|GetRollAmount) 0.01)
          (goto _label_3))))))

(fn CalculateSpeed
  (bind _physics_root (Variables|Default|GetPhysics%20Root))
  (bind _returnvalue (Physics|GetPhysicsLinearVelocity _physics_root "None"))
  (Physics|SetPhysicsLinearVelocity _physics_root (Math|Vector|Lerp(Vector) _returnvalue (* (Math|Vector|GetForwardVector _physics_root) (Math|Integer|Clamp(Integer) (* (Variables|Default|GetThrottleAmount) 100) 0 25000)) 0.01) false "None"))

(fn CalculateLift
  (bind _physics_root (Variables|Default|GetPhysics%20Root))
  ;[1 0 0.02566] TODO: lift based on forward velocity, not thrust
  (Physics|GetPhysicsLinearVelocity _physics_root "None")
  (Physics|AddForce _physics_root (* (Math|Vector|GetUpVector _physics_root) (Math|Conversions|ToFloat(Integer) (* (Variables|Default|GetThrottleAmount) 10))) "None" false))

(fn CheatForwardVelocity
  (bind _physics_root (Variables|Default|GetPhysics%20Root))
  (bind _forwardcheat (Variables|Default|GetForwardCheat))
  (bind _returnvalue (Physics|GetPhysicsLinearVelocity _physics_root "None"))
  (Physics|SetPhysicsLinearVelocity _physics_root (+ (* (Math|Vector|Normalize _returnvalue) (* (Math|Vector|VectorLength _returnvalue) (- 1.0 _forwardcheat))) (* (Math|Vector|GetForwardVector _physics_root) (* (Math|Vector|VectorLength _returnvalue) _forwardcheat))) false "None"))

(fn SettleTorque
  (bind _physics_root (Variables|Default|GetPhysics%20Root))
  (Class|PrimitiveComponent|AddTorqueinDegrees _physics_root (/ (Math|Vector|NegateVector (Physics|GetPhysicsAngularVelocityinDegrees _physics_root "None")) "0.500000,0.500000,0.500000") "None" true))

(fn SettleOrientation
  (bind _physics_root (Variables|Default|GetPhysics%20Root))
  (Class|PrimitiveComponent|AddTorqueinDegrees _physics_root (Math|Vector|Lerp(Vector) "0, 0, 0" (* (Math|Vector|GetForwardVector _physics_root) "") 0.1) "None" false))