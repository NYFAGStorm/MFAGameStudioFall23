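; Music_Trigger is a Blueprint that switches the game's music after a countdown.
; While TriggerCrossfade is set, Tick reduces TriggerTimer by delta time; nothing in this graph sets the flag.
; When the timer drops below zero, it clears the flag, finds the Music_Mgr actor by class and calls CrossfadeMusic with MusicSound.
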(event EventTick
  (params (DeltaSeconds :type Float%20%28single-precision%29))
  (if (Variables|Default|GetTrigger%20Crossfade)
    (bind _output_get (Variables|Default|SetTrigger%20Timer (- (Variables|Default|GetTrigger%20Timer) DeltaSeconds)))
    (if (< _output_get 0.0)
      (Variables|Default|SetTrigger%20Crossfade false)
      ;[0.3804 0.3294 0.2353] Code to Trigger New Music
      (bind _returnvalue (Actor|GetActorOfClass "/Game/Blueprint/BP_MusicManager/Music_Mgr.Music_Mgr_C"))
      (Default|CrossfadeMusic _returnvalue (Utilities|ResolveSoftReference (Variables|Default|GetMusic%20Sound))))))

(fn ConstructionScript)