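; Music manager Blueprint that loops background music on a primary audio component and crossfades to new tracks requested through CrossfadeMusic.
; Tick ramps the primary and secondary speaker volumes linearly in opposite directions while tracking the incoming track's playback position.
; When a fade ends or is interrupted by a new request, the secondary SoundWave moves to the primary speaker at that position, freeing the secondary for the next track.
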(event OnAudioFinished(PrimaryAudioSpeaker)
  ;[0.3804 0.3295 0.2355] Loop Primary Music
  (Audio|Components|Audio|Play (Variables|Default|GetPrimary%20Audio%20Speaker) 0.0))

(event EventTick
  (params (DeltaSeconds :type Float%20%28single-precision%29))
  ;[0.3804 0.3294 0.2353] Handle Crossfade Progress
  (if (Variables|Default|GetisCrossfading)
    (bind _output_get (Variables|Default|SetCrossfade%20Progress (+ (/ DeltaSeconds (Variables|Default|GetCrossfade%20Duration)) (Variables|Default|GetCrossfade%20Progress))))
    (Variables|Default|SetsecondaryPosition (+ DeltaSeconds (Variables|Default|GetsecondaryPosition)))
    (if (> _output_get 1.0)
      (CallFunction|CrossfadeEnd)
      (else
        (Utilities|FlowControl|Sequence
          (:then_0
            (Audio|Components|Audio|SetVolumeMultiplier (Variables|Default|GetPrimary%20Audio%20Speaker) (Math|Float|Clamp(Float) (- 1.0 _output_get)) :!class /Script/Engine.AudioComponent))
          (:then_1
            (Audio|Components|Audio|SetVolumeMultiplier (Variables|Default|GetSecondary%20Audio%20Speaker) (Math|Float|Clamp(Float) _output_get) :!class /Script/Engine.AudioComponent)))))))

(fn ConstructionScript)

(fn SetPrimaryMusic
  (params (New%20Sound :type Sound%20Wave%20Object%20Reference) (Start%20Time :type Float%20%28double-precision%29))
  (bind _primary_audio_speaker (Variables|Default|GetPrimary%20Audio%20Speaker))
  (Audio|Components|Audio|SetSound _primary_audio_speaker New%20Sound)
  (Audio|Components|Audio|SetVolumeMultiplier _primary_audio_speaker 1.0 :!class /Script/Engine.AudioComponent)
  (Audio|Components|Audio|Play _primary_audio_speaker Start%20Time))

(fn CrossfadeMusic
  (params (New%20Sound :type Sound%20Wave%20Object%20Reference))
  (bind _secondary_audio_speaker (Variables|Default|GetSecondary%20Audio%20Speaker))
  (if (Variables|Default|GetisCrossfading)
    ;[0.3804 0.3294 0.2353] Handle in-progress crossfade
    (bind _assound_wave (Utilities|Casting|CastToSoundWave (Variables|/Script/Engine.AudioComponent|GetSound _secondary_audio_speaker)))
    (CallFunction|SetPrimaryMusic _assound_wave (Variables|Default|GetsecondaryPosition)))
  (Audio|Components|Audio|SetSound _secondary_audio_speaker New%20Sound)
  (Audio|Components|Audio|SetVolumeMultiplier _secondary_audio_speaker 0.0 :!class /Script/Engine.AudioComponent)
  (Audio|Components|Audio|Play _secondary_audio_speaker 0.0)
  (Variables|Default|SetisCrossfading true)
  (Variables|Default|SetCrossfade%20Progress 0.0)
  (Variables|Default|SetsecondaryPosition 0.0))

(fn CrossfadeEnd
  (bind _secondary_audio_speaker (Variables|Default|GetSecondary%20Audio%20Speaker))
  (bind _assound_wave (Utilities|Casting|CastToSoundWave (Variables|/Script/Engine.AudioComponent|GetSound _secondary_audio_speaker))
    (:then
      (CallFunction|SetPrimaryMusic _assound_wave (Variables|Default|GetsecondaryPosition))
      (Audio|Components|Audio|Stop _secondary_audio_speaker)
      (Audio|Components|Audio|SetSound _secondary_audio_speaker 0)
      (Audio|Components|Audio|SetVolumeMultiplier _secondary_audio_speaker 0.0 :!class /Script/Engine.AudioComponent)
      (Variables|Default|SetisCrossfading false)
      (Variables|Default|SetCrossfade%20Progress 0.0))
    (:CastFailed
      (Development|PrintString "cannot cast from sound source to sound wave" true true "(R=1.000000,G=0.000000,B=0.627893,A=1.000000)"))))