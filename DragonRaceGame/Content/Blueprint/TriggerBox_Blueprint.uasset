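; Start/finish trigger box that counts laps and drives the race timer whenever something overlaps it.
; An active RingManager penalty check blocks the crossing; otherwise it increments the RaceTimer lap count and prints the lap time.
; The first crossing starts the timer, and later ones reset and restart it.
; Once laps exceed TotalLaps, it stops the timer and, after a short delay, reveals existing EndRaceHUD widgets.
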(event OnComponentBeginOverlap(CollisionComponent)
  (params (OverlappedComponent :type Primitive%20Component%20Object%20Reference) (OtherActor :type Actor%20Object%20Reference) (OtherComp :type Primitive%20Component%20Object%20Reference) (OtherBodyIndex :type Integer) (bFromSweep :type Boolean) (SweepResult :type Hit%20Result%20Structure%20%28by%20ref%29))
  (bind _racetimer (Variables|Default|GetRaceTimer))
  (bind _racetimer_2 (Variables|Default|GetRaceTimer))
  (bind _racetimer_3 (Variables|Default|GetRaceTimer))
  (if (Variables|/Game/Props/Prototype/Ring_Manager.Ring_Manager_C|GetPenalty%20Check (Variables|Default|GetRingManager))
    (Development|PrintText "Player has not finished the race")
    (elif (Utilities|IsValid (Variables|Default|GetRaceTimer))
      (bind _output_get (Variables|/Game/Blueprint/BP_RaceTimer/Race_Timer.Race_Timer_C|SetLaps _racetimer (+ (Variables|/Game/Blueprint/BP_RaceTimer/Race_Timer.Race_Timer_C|GetLaps _racetimer) 1 0)))
      (Development|PrintText (Utilities|Text|FormatText "Lap {LapNum}: {FormTime}" _output_get (Variables|/Game/Blueprint/BP_RaceTimer/Race_Timer.Race_Timer_C|GetFormTime _racetimer)) true true "(R=0.489583,G=0.000000,B=0.004675,A=1.000000)" 0.0)
      (Variables|/Game/Blueprint/BP_RaceTimer/Race_Timer.Race_Timer_C|SetRace%20Time _racetimer_3 0.0)
      (if (<= (Variables|/Game/Blueprint/BP_RaceTimer/Race_Timer.Race_Timer_C|GetLaps _racetimer_3) (Variables|Default|GettotalLaps))
        (if (> (Variables|/Game/Blueprint/BP_RaceTimer/Race_Timer.Race_Timer_C|GetLaps _racetimer_2) 1)
          (Default|ResetTimer _racetimer_2)
          (Default|StartTimer _racetimer_2)
          (Development|PrintText "Reset Time!")
          (else
            (Variables|/Game/Blueprint/BP_RaceTimer/Race_Timer.Race_Timer_C|SetisTimeRunning _racetimer_2 true)
            (Default|StartTimer _racetimer_2)
            (Development|PrintText "Race Started!")))
        (else
          (Variables|/Game/Blueprint/BP_RaceTimer/Race_Timer.Race_Timer_C|SetisTimeRunning _racetimer_2 false)
          (Development|PrintString "Race Complete!")
          (Utilities|FlowControl|Delay 1.0)
          (bind _foundwidgets (Widget|GetAllWidgetsOfClass "/Game/UI/HUD/EndRaceHUD.EndRaceHUD_C" true))
          (for _array_element _foundwidgets
            (Widget|SetVisibility _array_element "Visible"))))
      (else
        (Development|PrintString "Timer is missing")))))

(fn ConstructionScript)